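; BP_NarratorTrigger is a one-shot trigger volume that plays a narrator dialogue sound when the player enters it.
; Collision overlap by BP_MainPlayer plays DialogueToPlay at SoundLocation, then destroys the actor so the line cannot repeat.
; BeginPlay caches a Player reference through a GetPlayerMessage call on the player character, though the overlap logic never uses it.
; ToggleLight and the object query functions, such as GetObjectMass and IsObjectHeld, are empty or default-value stubs.
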(event OnComponentBeginOverlap(Collision)
  (params (OverlappedComponent :type Primitive%20Component%20Object%20Reference) (OtherActor :type Actor%20Object%20Reference) (OtherComp :type Primitive%20Component%20Object%20Reference) (OtherBodyIndex :type Integer) (bFromSweep :type Boolean) (SweepResult :type Hit%20Result%20Structure%20%28by%20ref%29))
  (Utilities|Casting|CastToBP_MainPlayer OtherActor)
  (Audio|PlaySoundatLocation (Variables|Default|GetDialogueToPlay) (Variables|Default|GetSoundLocation) "0, 0, 0" 1.0 1.0 0.0 0 0 0 0)
  (Actor|DestroyActor))

(event EventBeginPlay
  (bind _player (Class|BPIPlayerChecks|GetPlayer(Message) (Game|GetPlayerCharacter 0)))
  (Variables|Default|SetPlayer _player))

(event EventToggleLight)

(fn ConstructionScript)

(fn GetFPActor
  (return 0 0))

(fn GetObjectMass
  (return 0.0))

(fn GetTransitionVariables
  (return 0))

(fn IsObjectHeld
  (return false))