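; BP_SequencerManager is a level actor that plays the entrance and elevator cinematics and triggers the player's elevator respawn.
; BeginPlay caches the player's message reference and starts the entrance sequence.
; When BP_MainPlayer overlaps the collision, it plays the elevator sequence, waits briefly, then messages the player with the RespawnActor's respawn location transform.
; ToggleLight and the getter functions are empty or default-returning stubs.
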(event OnComponentBeginOverlap(Collision)
  (params (OverlappedComponent :type Primitive%20Component%20Object%20Reference) (OtherActor :type Actor%20Object%20Reference) (OtherComp :type Primitive%20Component%20Object%20Reference) (OtherBodyIndex :type Integer) (bFromSweep :type Boolean) (SweepResult :type Hit%20Result%20Structure%20%28by%20ref%29))
  (Utilities|Casting|CastToBP_MainPlayer OtherActor)
  (bind _returnvalue (Sequencer|Player|CreateLevelSequencePlayer (Variables|Default|GetElevatorSequence)))
  (Sequencer|Player|Play _returnvalue :!class /Script/MovieScene.MovieSceneSequencePlayer)
  (Utilities|FlowControl|Delay 3.0)
  (Class|BPIPlayerChecks|ElevatorRespawn(Message) (Variables|Default|GetPlayer) (Transformation|GetWorldTransform (Variables|/Game/Classes/Blueprints/InteractionSystem/Actors/Primary/BP_Elevator.BP_Elevator_C|GetRespawnLocation (Variables|Default|GetRespawnActor)))))

(event EventBeginPlay
  (bind _player (Class|BPIPlayerChecks|GetPlayer(Message) (Game|GetPlayerCharacter 0)))
  (Variables|Default|SetPlayer _player)
  (bind _returnvalue (Sequencer|Player|CreateLevelSequencePlayer (Variables|Default|GetEntranceSequence)))
  (Sequencer|Player|Play _returnvalue :!class /Script/MovieScene.MovieSceneSequencePlayer))

(event EventToggleLight)

(fn ConstructionScript)

(fn GetFPActor
  (return 0 0))

(fn GetObjectMass
  (return 0.0))

(fn GetTransitionVariables
  (return 0))

(fn IsObjectHeld
  (return false))