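; Player interactor component that lets the owning character detect and interact with interactable objects.
; Capsule begin and end overlaps message the other actor's AC_InteractableMaster and toggle the HUD overlay between hover and standard.
; Look input runs a line, forward-sphere or around-player trace, chosen by TraceType, and sets that overlay from the hit actor's Interactable tag.
; Interact input repeats the trace and sends CheckInteractionMessage to the hit component.
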(event Custom|HandleOnComponentOverlap
  (params (OverlappedComponent :type Primitive%20Component%20Object%20Reference) (OtherActor :type Actor%20Object%20Reference) (OtherComp :type Primitive%20Component%20Object%20Reference) (OtherBodyIndex :type Integer) (bFromSweep :type Boolean) (SweepResult :type Hit%20Result%20Structure%20%28by%20ref%29))
  (bind _returnvalue (Actor|GetComponentbyClass OtherActor "/Game/Classes/Blueprints/InteractionSystem/ComponentLibrary/Interactables/AC_InteractableMaster.AC_InteractableMaster_C"))
  ;[0 0 0] On Overlap - Check Relevant Interface And Call Interact Function
  (Class|BPIInteractionSystem|CheckInteraction(Message) _returnvalue "NewEnumerator2" "NewEnumerator0" (Variables|Components|GetCharacterRef) false self)
  (Utilities|IsValid _returnvalue
    (:Is%20Valid
      (Default|HoverUI (Variables|/Game/Classes/UI/BP_HUD.BP_HUD_C|GetWB_HUDOverlay (Variables|Default|GetBP_HUD))))))

(event Custom|HandleOnComponentOverlapEnd
  (params (OverlappedComponent :type Primitive%20Component%20Object%20Reference) (OtherActor :type Actor%20Object%20Reference) (OtherComp :type Primitive%20Component%20Object%20Reference) (OtherBodyIndex :type Integer))
  (bind _returnvalue (Actor|GetComponentbyClass OtherActor "/Game/Classes/Blueprints/InteractionSystem/ComponentLibrary/Interactables/AC_InteractableMaster.AC_InteractableMaster_C"))
  ;[0 0 0] On End Overlap - Check Relevant Interface And Call Interact Function
  (Class|BPIInteractionSystem|CheckInteraction(Message) _returnvalue "NewEnumerator5" "NewEnumerator0" (Variables|Components|GetCharacterRef) false self)
  (Utilities|IsValid _returnvalue
    (:Is%20Valid
      (Default|StandardUI (Variables|/Game/Classes/UI/BP_HUD.BP_HUD_C|GetWB_HUDOverlay (Variables|Default|GetBP_HUD))))))

(event Input|EnhancedActionEvents|EnhancedInputActionIA_StandardInteract
  (params (ActionValue :type Boolean) (ElapsedSeconds :type Float%20%28double-precision%29) (TriggeredSeconds :type Float%20%28double-precision%29) (InputAction :type Input%20Action%20Object%20Reference :default "/Game/Classes/Input/Actions/IA_StandardInteract.IA_StandardInteract"))
  (bind _self self)
  (bind _cameracomp (Variables|Default|GetCameraComp))
  (bind _cameracomp_2 (Variables|Default|GetCameraComp))
  ;[0 0 0] Switch on trace type change in EUW_Base - calls component macro library traces - If Interface is found, call interact function
  (:Started
    (switch Utilities|FlowControl|Switch|SwitchonE_TraceType (Variables|AdvancedConfig|GetTraceType)
      (:NewEnumerator9
        (bind _hitcomp (Utilities|BasicLineForward _cameracomp _cameracomp (Variables|AdvancedConfig|GetTrace%20Length) (Variables|AdvancedConfig|GetDraw%20Debug%20Type))
          (:true
            (Class|BPIInteractionSystem|CheckInteraction(Message) _hitcomp "NewEnumerator3" "NewEnumerator11" (Variables|Components|GetCharacterRef) false _self))))
      (:NewEnumerator7
        (bind _hitcomp_2 (Utilities|SphereTraceForward _cameracomp_2 _cameracomp_2 (Variables|AdvancedConfig|GetTrace%20Radius) (Variables|AdvancedConfig|GetTrace%20Length) (Variables|AdvancedConfig|GetDraw%20Debug%20Type))
          (:true
            (Class|BPIInteractionSystem|CheckInteraction(Message) _hitcomp_2 "NewEnumerator3" "NewEnumerator11" (Variables|Components|GetCharacterRef) false _self))))
      (:NewEnumerator8
        (bind _hitcomp_3 (Utilities|SphereTraceAroundPlayer (Variables|Default|GetCameraComp) (Variables|AdvancedConfig|GetTrace%20Radius) (Variables|AdvancedConfig|GetDraw%20Debug%20Type))
          (:true
            (Class|BPIInteractionSystem|CheckInteraction(Message) _hitcomp_3 "NewEnumerator3" "NewEnumerator11" (Variables|Components|GetCharacterRef) false _self)))))))

(event Input|EnhancedActionEvents|EnhancedInputActionIA_Look
  (params (ActionValue :type Vector%202D%20Structure) (ElapsedSeconds :type Float%20%28double-precision%29) (TriggeredSeconds :type Float%20%28double-precision%29) (InputAction :type Input%20Action%20Object%20Reference :default "/Game/Classes/Input/Actions/IA_Look.IA_Look"))
  (bind _cameracomp (Variables|Default|GetCameraComp))
  (bind _cameracomp_2 (Variables|Default|GetCameraComp))
  (switch Utilities|FlowControl|Switch|SwitchonE_TraceType (Variables|AdvancedConfig|GetTraceType)
    (:NewEnumerator9
      (bind _hitactor (Utilities|BasicLineForward _cameracomp_2 _cameracomp_2 (Variables|AdvancedConfig|GetTrace%20Length) (Variables|AdvancedConfig|GetDraw%20Debug%20Type))
        (:true
          (if (Actor|ActorHasTag _hitactor "Interactable")
            (Default|HoverUI (Variables|/Game/Classes/UI/BP_HUD.BP_HUD_C|GetWB_HUDOverlay (Variables|Default|GetBP_HUD)) :!label _label)
            (else
              (Default|StandardUI (Variables|/Game/Classes/UI/BP_HUD.BP_HUD_C|GetWB_HUDOverlay (Variables|Default|GetBP_HUD)) :!label _label_2))))))
    (:NewEnumerator7
      (bind _hitactor_2 (Utilities|SphereTraceForward _cameracomp _cameracomp (Variables|AdvancedConfig|GetTrace%20Radius) (Variables|AdvancedConfig|GetTrace%20Length) (Variables|AdvancedConfig|GetDraw%20Debug%20Type))
        (:true
          (if (Actor|ActorHasTag _hitactor_2 "Interactable")
            (goto _label)
            (else
              (goto _label_2))))))
    (:NewEnumerator8
      (bind _hitactor_3 (Utilities|SphereTraceAroundPlayer (Variables|Default|GetCameraComp) (Variables|AdvancedConfig|GetTrace%20Radius) (Variables|AdvancedConfig|GetDraw%20Debug%20Type))
        (:true
          (if (Actor|ActorHasTag _hitactor_3 "Interactable")
            (goto _label)
            (else
              (goto _label_2))))))))

(event EventBeginPlay
  ;[0 0 1] Begin Play
  (bind _ascharacter (Utilities|Casting|CastToCharacter (Components|GetOwner)))
  (Variables|Components|SetCharacterRef _ascharacter)
  (Collision|BindEventtoOnComponentBeginOverlap (Variables|/Script/Engine.Character|GetCapsuleComponent _ascharacter) (EventDispatchers|CreateEvent :!event Custom|HandleOnComponentOverlap))
  (Collision|BindEventtoOnComponentEndOverlap (Variables|/Script/Engine.Character|GetCapsuleComponent _ascharacter) (EventDispatchers|CreateEvent :!event Custom|HandleOnComponentOverlapEnd))
  (CallFunction|FetchClasses))

(fn GetTracePointRef
  (params (Trace%20Comp :type Primitive%20Component%20Object%20Reference) (Camera%20Comp :type Camera%20Component%20Object%20Reference))
  (bind _output_get (Variables|Default|SetTraceComp Trace%20Comp))
  (bind _output_get_2 (Variables|Default|SetCameraComp Camera%20Comp))
  (return _output_get _output_get_2))

(fn GetComponent
  (params (ComponentToQuery :type Actor%20Component%20Class%20Reference) (Querier :type Actor%20Object%20Reference)))

(fn FetchClasses
  (bind _asbp_hud (Utilities|Casting|CastToBP_HUD (HUD|GetHUD (Game|GetPlayerController 0))))
  (Variables|Default|SetBP_HUD _asbp_hud))

(fn GetTraceLength
  (return (Variables|AdvancedConfig|GetTrace%20Length)))