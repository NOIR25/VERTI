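; Actor component in the interaction system that lets its owning actor act as an interactor through overlaps.
; On BeginPlay it gets the interactor and overlap component from the owner, then binds begin and end overlap events.
; Both handlers pass a distinct interaction type to the other actor's AC_InteractableMaster via CheckInteractionMessage.
; Small functions expose trace component, camera and trace length, while GetComponent is an empty stub.
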(event Custom|HandleOnComponentOverlap
  (params (OverlappedComponent :type Primitive%20Component%20Object%20Reference) (OtherActor :type Actor%20Object%20Reference) (OtherComp :type Primitive%20Component%20Object%20Reference) (OtherBodyIndex :type Integer) (bFromSweep :type Boolean) (SweepResult :type Hit%20Result%20Structure%20%28by%20ref%29))
  ;[0 0 0] On Overlap - Check Relevant Interface And Call Interact Function
  (Class|BPIInteractionSystem|CheckInteraction(Message) (Actor|GetComponentbyClass OtherActor "/Game/Classes/Blueprints/InteractionSystem/ComponentLibrary/Interactables/AC_InteractableMaster.AC_InteractableMaster_C") "NewEnumerator2" "NewEnumerator0" (Variables|Default|GetActor%20Interactor) false self))

(event Custom|HandleOnComponentOverlapEnd
  (params (OverlappedComponent :type Primitive%20Component%20Object%20Reference) (OtherActor :type Actor%20Object%20Reference) (OtherComp :type Primitive%20Component%20Object%20Reference) (OtherBodyIndex :type Integer))
  ;[0 0 0] On End Overlap - Check Relevant Interface And Call Interact Function
  (Class|BPIInteractionSystem|CheckInteraction(Message) (Actor|GetComponentbyClass OtherActor "/Game/Classes/Blueprints/InteractionSystem/ComponentLibrary/Interactables/AC_InteractableMaster.AC_InteractableMaster_C") "NewEnumerator5" "NewEnumerator0" (Variables|Default|GetActor%20Interactor) false self))

(event EventBeginPlay
  ;[0 0 1] Begin Play
  (bind (_actorinteractor _overlapcomp) (Class|BPIPlayerChecks|GetActorInteractor(Message) (Components|GetOwner)))
  (Variables|Default|SetActor%20Interactor _actorinteractor)
  (bind _output_get (Variables|Default|SetOverlap%20Comp _overlapcomp))
  (Collision|BindEventtoOnComponentBeginOverlap _output_get (EventDispatchers|CreateEvent :!event Custom|HandleOnComponentOverlap))
  (Collision|BindEventtoOnComponentEndOverlap _output_get (EventDispatchers|CreateEvent :!event Custom|HandleOnComponentOverlapEnd)))

(fn GetTracePointRef
  (params (Trace%20Comp :type Primitive%20Component%20Object%20Reference) (Camera%20Comp :type Camera%20Component%20Object%20Reference))
  (bind _output_get (Variables|Default|SetTraceComp Trace%20Comp))
  (bind _output_get_2 (Variables|Default|SetCameraComp Camera%20Comp))
  (return _output_get _output_get_2))

(fn GetComponent
  (params (ComponentToQuery :type Actor%20Component%20Class%20Reference) (Querier :type Actor%20Object%20Reference)))

(fn GetTraceLength
  (return (Variables|AdvancedConfig|GetTrace%20Length)))