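; Door behaviour component in the interaction system that lets its owning actor respond to interactions as a door.
; It extends a parent interactable component, calling the parent version of each overridden event first.
; Direct interaction and chained triggers both send OpenDoorMessage to the owner, leaving the actual opening to that actor.
; Begin, overlap and end-overlap events add only debug prints.
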(event EventBeginPlay
  (|CallParentFunction))

(event EventTick
  (params (DeltaSeconds :type Float%20%28single-precision%29)))

(fn EventInteract
  (params (Interactor :type Actor%20Object%20Reference) (AltInput :type Boolean))
  (|CallParentFunction 0 false)
  (Class|BPIBehaviours|OpenDoor(Message) (Variables|Default|GetOwner)))

(fn EventBeginPlay
  (|CallParentFunction)
  (Development|PrintString "Begin Event - Door"))

(fn EventChained
  (params (Interactor :type Actor%20Object%20Reference))
  (|CallParentFunction 0)
  (Class|BPIBehaviours|OpenDoor(Message) (Variables|Default|GetOwner)))

(fn EventOverlap
  (params (Interactor :type Actor%20Object%20Reference))
  (|CallParentFunction 0)
  (Development|PrintString "Overlap Event - Door"))

(fn EventEndOverlap
  (params (Interactor :type Actor%20Object%20Reference))
  (|CallParentFunction 0)
  (Development|PrintString "End Overlap Event - Door"))