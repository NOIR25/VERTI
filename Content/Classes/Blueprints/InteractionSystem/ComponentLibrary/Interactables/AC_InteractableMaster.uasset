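; Base actor component for interactables in the interaction system, with empty event functions as hooks for specific behaviours.
; CheckInteraction matches the interaction type against CallType and checks input behaviour, then sends the matching overlap, end-overlap, interact or chained-event message.
; Event handlers wait TimeBeforeSelfEvent before calling their hooks, as does BeginPlay when CallType includes it.
; A loop forwarding chained events to ChainTo actors exists but is unconnected.
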(event EventBeginPlay
  (bind _returnvalue (Components|GetOwner))
  (Utilities|IsValid _returnvalue
    (:Is%20Valid
      (Variables|Default|SetOwner _returnvalue)
      (for _array_element (Variables|ActionBlocks|GetCallType)
        (if (Utilities|Enum|Equal(Enum) _array_element "NewEnumerator6")
          (Utilities|DelayEvent (Variables|ActionBlocks|GetTimeBefore%28Self%29Event)
            (:Completed
              (CallFunction|EventBeginPlay))))))
    (:Is%20Not%20Valid
      (if (Utilities|Enum|Equal(Enum) _array_element "NewEnumerator6")
        (Utilities|DelayEvent (Variables|ActionBlocks|GetTimeBefore%28Self%29Event)
          (:Completed
            (CallFunction|EventBeginPlay)))))))

(event EventCheckInteraction
  (params (InteractionType :type E_EventCallType%20Enum :default "NewEnumerator0") (InputBehaviour :type E_PressType%20Enum :default "NewEnumerator0") (Interactor :type Actor%20Object%20Reference) (Alt%20Input :type Boolean) (InteractorComponent :type Actor%20Component%20Object%20Reference))
  (bind _self self)
  (Variables|Default|SetAlt%20Input Alt%20Input)
  (Variables|Default|SetInteractor%20Component InteractorComponent)
  (Variables|Default|SetInteractor Interactor)
  (Utilities|CheckInteractionInputs InteractionType InputBehaviour
    (:true
      (switch Utilities|FlowControl|Switch|SwitchonE_EventCallType InteractionType
        (:NewEnumerator2
          (Class|BPIInteractionSystem|Overlap(Message) _self (Variables|Default|GetInteractor) (Variables|Default|GetAlt%20Input)))
        (:NewEnumerator5
          (Class|BPIInteractionSystem|EndOverlap(Message) _self (Variables|Default|GetInteractor) (Variables|Default|GetAlt%20Input)))
        (:NewEnumerator3
          (Class|BPIInteractionSystem|Interact(Message) _self (Variables|Default|GetInteractor) (Variables|Default|GetAlt%20Input)))
        (:NewEnumerator4
          (Class|BPIInteractionSystem|ChainedEvent(Message) _self (Variables|Default|GetInteractor) (Variables|Default|GetAlt%20Input)))))
    (:false
      (Development|PrintString "Interaction Failed - Input Or Behaviour Does Not Match" true true "(R=1.000000,G=0.000000,B=0.000000,A=1.000000)" 2.0 "Error"))))

(event EventOverlap
  (params (Interactor :type Actor%20Object%20Reference) (AltInput :type Boolean))
  (Utilities|DelayEvent (Variables|ActionBlocks|GetTimeBefore%28Self%29Event)
    (:Completed
      (CallFunction|EventOverlap Interactor))))

(event EventInteract
  (params (Interactor :type Actor%20Object%20Reference) (AltInput :type Boolean))
  (Utilities|DelayEvent (Variables|ActionBlocks|GetTimeBefore%28Self%29Event)
    (:Completed
      (CallFunction|EventInteract Interactor AltInput))))

(event EventEndOverlap
  (params (Interactor :type Actor%20Object%20Reference) (AltInput :type Boolean))
  (Utilities|DelayEvent (Variables|ActionBlocks|GetTimeBefore%28Self%29Event)
    (:Completed
      (CallFunction|EventEndOverlap Interactor))))

(event EventChainedEvent
  (params (Interactor :type Actor%20Object%20Reference) (AltInput :type Boolean))
  (Utilities|DelayEvent (Variables|ActionBlocks|GetTimeBefore%28Self%29Event)
    (:Completed
      (CallFunction|EventChained Interactor))))

(fn EventInteract
  (params (Interactor :type Actor%20Object%20Reference) (AltInput :type Boolean)))

(fn EventOverlap
  (params (Interactor :type Actor%20Object%20Reference)))

(fn EventEndOverlap
  (params (Interactor :type Actor%20Object%20Reference)))

(fn EventChained
  (params (Interactor :type Actor%20Object%20Reference)))

(fn EventBeginPlay)