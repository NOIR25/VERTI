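; Interactable behaviour component for lights in the interaction system, telling its owning actor to toggle its light.
; It overrides the parent's begin play, interact, chained, overlap and end-overlap events, each calling the parent and then sending a Toggle Light message to the owner.
; The component holds no light state or logic, leaving the actual switching to the owner.
; The interact override passes AltInput to the parent as false.
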(event EventBeginPlay
  (|CallParentFunction) ; This node is disabled and will not be called.\nDrag off pins to build functionality.
)

(event EventTick
  (params (DeltaSeconds :type Float%20%28single-precision%29)))

(fn EventBeginPlay
  (|CallParentFunction)
  (Class|BPIBehaviours|ToggleLight(Message) (Variables|Default|GetOwner)))

(fn EventChained
  (params (Interactor :type Actor%20Object%20Reference))
  (|CallParentFunction 0)
  (Class|BPIBehaviours|ToggleLight(Message) (Variables|Default|GetOwner)))

(fn EventEndOverlap
  (params (Interactor :type Actor%20Object%20Reference))
  (|CallParentFunction 0)
  (Class|BPIBehaviours|ToggleLight(Message) (Variables|Default|GetOwner)))

(fn EventInteract
  (params (Interactor :type Actor%20Object%20Reference) (AltInput :type Boolean))
  (|CallParentFunction 0 false)
  (Class|BPIBehaviours|ToggleLight(Message) (Variables|Default|GetOwner)))

(fn EventOverlap
  (params (Interactor :type Actor%20Object%20Reference))
  (|CallParentFunction 0)
  (Class|BPIBehaviours|ToggleLight(Message) (Variables|Default|GetOwner)))