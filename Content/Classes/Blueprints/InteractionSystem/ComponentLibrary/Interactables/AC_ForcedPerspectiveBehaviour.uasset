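; AC_ForcedPerspectiveBehaviour is an interactable component that routes interactions for forced-perspective objects the interactor can hold.
; Its EventInteract override runs the parent logic, then sends a match-scale message to the owner on alternate input.
; Normal input toggles the interactor's holding state and tells the owner to pick up or drop.
; All calls go through messages, leaving the scaling and carrying logic outside this component.
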(event EventBeginPlay
  (|CallParentFunction) ; This node is disabled and will not be called.\nDrag off pins to build functionality.
)

(event EventTick
  (params (DeltaSeconds :type Float%20%28single-precision%29)))

(fn EventInteract
  (params (Interactor :type Actor%20Object%20Reference) (AltInput :type Boolean))
  (|CallParentFunction Interactor AltInput)
  (if AltInput
    (Class|BPIBehaviours|MatchScale(Message) (Variables|Default|GetOwner) (Variables|Default|GetInteractor) (Variables|Default|GetInteractor%20Component))
    (else
      (bind _holding (Class|BPIPlayerChecks|IsHoldingObject(Message) Interactor))
      (if _holding
        (Class|BPIPlayerChecks|SetIsHoldingObject(Message) (Variables|Default|GetInteractor) false)
        (Class|BPIBehaviours|DropObject(Message) (Variables|Default|GetOwner))
        (else
          (Class|BPIPlayerChecks|SetIsHoldingObject(Message) (Variables|Default|GetInteractor) true)
          (Class|BPIBehaviours|PickupObject(Message) (Variables|Default|GetOwner) (Variables|Default|GetInteractor) (Variables|Default|GetInteractor%20Component)))))))