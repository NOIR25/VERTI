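; BP_Elevator is an elevator actor in the interaction system, though this file holds no movement logic.
; Its construction script caches the world locations of the CameraStart and RespawnLocation components into WorldCamLocation and RespawnLoc.
; The functions for first-person actor, object mass, transition variables and held state are stubs that return nothing or default values.
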(fn ConstructionScript
  (Variables|Default|SetWorldCamLocation (Transformation|GetWorldLocation (Variables|Default|GetCameraStart)))
  (Variables|Default|SetRespawnLoc (Transformation|GetWorldLocation (Variables|Default|GetRespawnLocation))))

(fn GetFPActor
  (return 0 0))

(fn GetObjectMass
  (return 0.0))

(fn GetTransitionVariables
  (return 0))

(fn IsObjectHeld
  (return false))