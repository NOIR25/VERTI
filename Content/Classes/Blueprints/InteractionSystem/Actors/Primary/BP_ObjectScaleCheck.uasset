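; Puzzle trigger that checks whether an overlapping FP object has been scaled to a required size, then unlocks a chained actor.
; While the object overlaps, a looping timer compares its Z scale to the target within an assist tolerance.
; On a match it drops the object, then a timeline lerps it to the chained component's location and required scale with physics and collision disabled.
; When finished, it destroys the object and sends the unlock interface message.
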(event OnComponentBeginOverlap(Collision)
  (params (OverlappedComponent :type Primitive%20Component%20Object%20Reference) (OtherActor :type Actor%20Object%20Reference) (OtherComp :type Primitive%20Component%20Object%20Reference) (OtherBodyIndex :type Integer) (bFromSweep :type Boolean) (SweepResult :type Hit%20Result%20Structure%20%28by%20ref%29))
  ;[0 0 0] Overlap with FP actor - Check validity - If success start timer
  (bind (_component _actor) (Class|BPIBehaviours|GetFPActor(Message) OtherActor))
  (bind _output_get (Variables|Default|SetFP%20Component _component))
  (Variables|Actors|SetActor _actor)
  (Utilities|IsValid _output_get
    (:Is%20Valid
      (bind _returnvalue (Utilities|Time|SetTimerbyEvent (EventDispatchers|CreateEvent :!event Custom|CE_CheckScale) 0.1 true))
      (Variables|Timer|SetScaleCheckTimer _returnvalue))))

(event OnComponentEndOverlap(Collision)
  (params (OverlappedComponent :type Primitive%20Component%20Object%20Reference) (OtherActor :type Actor%20Object%20Reference) (OtherComp :type Primitive%20Component%20Object%20Reference) (OtherBodyIndex :type Integer))
  ;[0 0 0] End overlap - Clear timer
  (Utilities|Time|ClearandInvalidateTimerbyHandle (Variables|Timer|GetScaleCheckTimer)))

(event Custom|CE_CheckScale
  ;[0 0 0] Check scale is nearly = to our the requirement - Allow error tolerance for more assisted play - If success, drop object and stop timer
  (bind _output_get (Variables|Float|SetCurrentObjectScale (.z (Transformation|GetWorldScale (Variables|Default|GetFP%20Component)))))
  (if (Math|Float|NearlyEqual(Float) _output_get (Variables|Float|GetRequiredScale) (Variables|Float|GetErrorTolerance))
    (Class|BPIBehaviours|DropObject(Message) (Variables|Actors|GetActor))
    (CallFunction|CEStopChecks)))

(event Custom|CE_StopChecks
  ;[0 0 0] Stop checks clear timer
  (Utilities|Time|ClearandInvalidateTimerbyHandle (Variables|Timer|GetScaleCheckTimer))
  (CallFunction|CELerpActor))

(event Custom|CE_LerpActor
  (bind _chainto (Variables|Actors|GetChainTo))
  (bind _fp_component (Variables|Default|GetFP%20Component))
  (bind _fp_component_2 (Variables|Default|GetFP%20Component))
  (bind _returnvalue (Transformation|GetWorldTransform _fp_component))
  ;[0 0 0] Lerp actor to desired location - disables physics and collisions to prevent errors
  (Utilities|IsValid (Variables|Default|GetCopy%20Component)
    (:Is%20Valid
      (bind _alpha (Timeline|LerpActor PlayFromStart)
        (:Update
          (Transformation|SetWorldTransform _fp_component_2 (Math|Transform|MakeTransform (Math|Vector|Lerp(Vector) (.location _returnvalue) (Transformation|GetWorldLocation (Variables|Default|GetCopy%20Component)) _alpha) (.rotation _returnvalue) (Math|Vector|Lerp(Vector) (.scale _returnvalue) (Variables|Vectors|GetRequiredScaleVector) _alpha)) false false)
          (Physics|SetSimulatePhysics _fp_component_2 false)
          (Collision|SetCollisionEnabled _fp_component_2 "NoCollision"))
        (:Finished
          ;[0 0 0] Call unlock and destroy the scaling actor
          (Actor|DestroyActor (Variables|Actors|GetActor))
          (Utilities|IsValid _chainto
            (:Is%20Valid
              (Class|BPIBehaviours|TriggerUnlock(Message) _chainto))))))))

(event EventBeginPlay
  ;[0 0 0] Set base variables via interface pointing to the chained actor
  (Variables|Float|SetRequiredScale (.z (Variables|Vectors|GetRequiredScaleVector)))
  (bind _copycomponent (Class|BPIBehaviours|GetTransitionVariables(Message) (Variables|Actors|GetChainTo)))
  (Variables|Default|SetCopy%20Component _copycomponent))

(fn ConstructionScript)

(fn GetFPActor
  (return 0 0))

(fn GetObjectMass
  (return 0.0))

(fn GetTransitionVariables)

(fn IsObjectHeld
  (return false))