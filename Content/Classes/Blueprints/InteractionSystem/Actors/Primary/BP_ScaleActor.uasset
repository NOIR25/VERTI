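; BP_ScaleActor is an interactable that resizes whoever interacts with it to match the scale of its Box.
; Construction caches the Box's world scale as the target.
; PickupObject plays a one-time sound and, unless held, runs a timeline lerping the interactor's scale component from its current scale toward that target, with clamped vector size.
; It exposes itself, Collision and Box through interaction getters; most others are stubs.
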(event EventPickupObject
  (params (Interactor :type Actor%20Object%20Reference) (InteractorComponent :type Actor%20Component%20Object%20Reference))
  ;[0 0 0] Match Player Scale To Object
  (Utilities|FlowControl|Sequence
    (:then_0
      (Utilities|FlowControl|DoOnce false
        (:Completed
          (Audio|PlaySound2D (Variables|Editable|GetSoundToPlay) 1.0 1.0 0.0 0 0))))
    (:then_1
      (if (not (Variables|Validation|GetisHeld))
        (bind _scalecomponent (Class|BPIPlayerChecks|GetScaleComponent(Message) Interactor))
        (Variables|Default|SetScale%20Component _scalecomponent)
        (Variables|Default|SetInteractor%20Component InteractorComponent)
        (bind _alpha (Timeline|Timeline PlayFromStart)
          (:Update
            (Transformation|SetWorldScale3D (Variables|Default|GetScale%20Component) (Math|Vector|ClampVectorSize (Math|Vector|Lerp(Vector) (Transformation|GetWorldScale (Variables|Default|GetScale%20Component)) (Variables|Vectors|GetFinalScale) _alpha) 0.1 2.0))))))))

(fn ConstructionScript
  (CallFunction|GetScale))

(fn GetScale
  (Variables|Vectors|SetFinalScale (Transformation|GetWorldScale (Variables|Default|GetBox))))

(fn GetActorInteractor
  (return self (Variables|Default|GetCollision)))

(fn GetFPActor
  (return (Variables|Default|GetBox) self))

(fn GetObjectMass
  (return 0.0))

(fn GetPhysicsHandle
  (return 0))

(fn GetPickupComponent
  (return 0))

(fn GetPlayer
  (return 0))

(fn GetScaleComponent
  (return 0))

(fn GetTransitionVariables
  (return 0))

(fn IsHoldingObject
  (return false))

(fn IsObjectHeld
  (return (Variables|Validation|GetisHeld)))

(fn SetHeldObject
  (params (Component :type Primitive%20Component%20Object%20Reference))
  (return 0))