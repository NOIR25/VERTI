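; Door frame in the interaction system that stays blocked by a wall until an unlock trigger accepts the puzzle solution.
; The toggle event swaps visibility and collision between BlockingWall and Door; unblocking also opens the door.
; Opening plays a confirmation sound while a timeline lerps yaw from its current value toward a fixed angle.
; Interaction getters expose DoorPositionActor for transitions and otherwise return empty, non-held defaults.
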(event Custom|CE_ToggleBlock
  (params (Block :type Boolean))
  (bind _blockingwall (Variables|Default|GetBlockingWall))
  (bind _door (Variables|Default|GetDoor))
  (bind _blockingwall_2 (Variables|Default|GetBlockingWall))
  (bind _door_2 (Variables|Default|GetDoor))
  ;[0 0 0] Trigger unblock - accept puzzle solution
  (if Block
    (Rendering|SetVisibility _blockingwall true false)
    (Collision|SetCollisionEnabled _blockingwall "QueryAndPhysics")
    (Rendering|SetVisibility _door_2 false false)
    (Collision|SetCollisionEnabled _door_2 "NoCollision")
    (else
      (Rendering|SetVisibility _blockingwall_2 false false)
      (Collision|SetCollisionEnabled _blockingwall_2 "NoCollision")
      (Rendering|SetVisibility _door true false)
      (Collision|SetCollisionEnabled _door "QueryAndPhysics")
      (CallFunction|CEOpenDoor))))

(event Custom|CE_OpenDoor
  (bind _door (Variables|Default|GetDoor))
  (bind _relativerotation (Variables|/Script/Engine.SceneComponent|GetRelativeRotation _door))
  ;[0 0 0] Open Door
  (Audio|PlaySoundatLocation "/Game/Assets/SFX/general/Beeps/Correct_Cue.Correct_Cue" (Transformation|GetWorldLocation (Variables|Default|GetFrame)) "0, 0, 0" 1.0 1.0 0.0 0 0 0 0)
  (bind _alpha (Timeline|DoorOpen PlayFromStart)
    (:Update
      (Transformation|SetRelativeRotation _door (Math|Rotator|MakeRotator (.roll _relativerotation) (.pitch _relativerotation) (Math|Float|Lerp (.yaw _relativerotation) -9e+01 _alpha)) false false))))

(event EventTriggerUnlock
  ;[0 0 0] Call trigger unblock
  (CallFunction|CEToggleBlock false))

(fn ConstructionScript)

(fn GetFPActor
  (return 0 0))

(fn GetObjectMass
  (return 0.0))

(fn GetTransitionVariables
  (return (Variables|Default|GetDoorPositionActor)))

(fn IsObjectHeld
  (return false))