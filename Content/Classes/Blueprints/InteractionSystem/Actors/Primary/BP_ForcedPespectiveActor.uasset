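; Pickup actor for forced-perspective puzzles: a held object moves out to the nearest surface behind it and rescales by distance, keeping its apparent size.
; While held, a gated looping timer line-traces through the vertices of a low-poly proxy mesh to find the closest hit.
; A timeline eases the object toward view center, with optional rotation alignment.
; Dropping restores physics and applies mass multiplied by the final scale.
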(event Custom|Smooth%20Transition
  ;[0 0 0] Drop Object
  (Utilities|FlowControl|DoOnce false
    (:Completed
      (bind _alpha (Timeline|Timeline_0 PlayFromStart)
        (:Update
          (Variables|ForcedPerspective|SetTransitionAlpha _alpha))))))

(event Custom|CE_AlignToOriginalOrientation
  ;[0 0 0] Align to original orientation
  (bind _alpha (Timeline|AlignOrientation PlayFromStart)
    (:Update
      (Variables|Validation|SetAligning true)
      (Transformation|SetWorldRotation (Variables|Default|GetBox) (Math|Rotator|Lerp(Rotator) (Transformation|GetWorldRotation (Variables|Default|GetBox)) "0, 0, 0" _alpha) false false))
    (:Finished
      (Variables|Validation|SetAligning false))))

(event Custom|CE_ScaleFP
  ;[0 0 0] Gate - Controls forced perspective activation and deactivation
  (Utilities|FlowControl|Gate true
    (:Exit
      (CallFunction|CustomVertexTrace))))

(event Custom|CE_AlignToOrigin
  (params (StartingLocation :type Vector))
  ;[0 0 0] Align To Origin
  (bind _alpha (Timeline|AlignToOrigin PlayFromStart)
    (:Update
      (Transformation|SetRelativeLocation (Variables|Default|GetBox) (Math|Vector|Lerp(Vector) StartingLocation (* (Math|Vector|Distance(Vector) "0, 0, 0" StartingLocation) "1.000000,0.000000,0.000000") _alpha) false true))
    (:Finished
      (CallFunction|CEOpenGate))))

(event Custom|CE_OpenGate
  ;[0 0 0] Gate - Controls forced perspective activation and deactivation
  (Utilities|FlowControl|Gate true) ; enters at Open
)

(event Custom|CE_CloseGate
  ;[0 0 0] Gate - Controls forced perspective activation and deactivation
  (Utilities|FlowControl|Gate true) ; enters at Close
)

(event Input|EnhancedActionEvents|EnhancedInputActionIA_StandardInteract
  (params (ActionValue :type Boolean) (ElapsedSeconds :type Float%20%28double-precision%29) (TriggeredSeconds :type Float%20%28double-precision%29) (InputAction :type Input%20Action%20Object%20Reference :default "/Game/Classes/Input/Actions/IA_StandardInteract.IA_StandardInteract"))
  (bind _box (Variables|Default|GetBox))
  ;[0 0 0] Drop Object
  (:Started
    (Input|DisableInput (Game|GetPlayerController 0))
    (Class|BPIPlayerChecks|SetHeldObject(Message) (Variables|Classes|GetInteractor))
    (Transformation|DetachFromComponent _box "KeepWorld" "KeepWorld" "KeepWorld" true)
    (Collision|SetCollisionEnabled _box "QueryAndPhysics")
    (Physics|SetSimulatePhysics _box true)
    (CallFunction|CECloseGate)
    (Variables|Validation|SetisHeld false)
    (CallFunction|SetMass)
    (Utilities|Time|ClearandInvalidateTimerbyHandle (Variables|Timers|GetSFP_Timer))
    (Utilities|FlowControl|DoOnce false) ; enters at Reset
  ))

(event EventDropObject
  (bind _box (Variables|Default|GetBox))
  ;[0 0 0] Drop Object
  (Input|DisableInput (Game|GetPlayerController 0))
  (Class|BPIPlayerChecks|SetHeldObject(Message) (Variables|Classes|GetInteractor))
  (Transformation|DetachFromComponent _box "KeepWorld" "KeepWorld" "KeepWorld" true)
  (Collision|SetCollisionEnabled _box "QueryAndPhysics")
  (Physics|SetSimulatePhysics _box true)
  (CallFunction|CECloseGate)
  (Variables|Validation|SetisHeld false)
  (CallFunction|SetMass)
  (Utilities|Time|ClearandInvalidateTimerbyHandle (Variables|Timers|GetSFP_Timer))
  (Utilities|FlowControl|DoOnce false) ; enters at Reset
)

(event EventBeginPlay
  ;[0 0 0] Get Starting Mass
  (CallFunction|GetMass))

(event EventPickupObject
  (params (Interactor :type Actor%20Object%20Reference) (InteractorComponent :type Actor%20Component%20Object%20Reference))
  (bind _box (Variables|Default|GetBox))
  ;[0 0 0] Pickup Object
  (Utilities|FlowControl|Sequence
    (:then_0
      (Utilities|FlowControl|DoOnce false
        (:Completed
          (Audio|PlaySound2D (Variables|Editable|GetSound%20To%20Play) 1.0 1.0 0.0 0 0))))
    (:then_1
      (CallFunction|GetPickupBaseVariables Interactor InteractorComponent)
      (Transformation|AttachComponentToComponent (Variables|Default|GetBox) (Variables|Default|GetParent%20Component) "None" "KeepWorld" "KeepWorld" "KeepWorld" true)
      (Physics|SetSimulatePhysics _box false)
      (Collision|SetCollisionEnabled _box "NoCollision")
      (CallFunction|GetStartVariables)
      (switch Utilities|FlowControl|Switch|SwitchonE_ScalingTypes (Variables|Editable|GetScaleTypes)
        (:NewEnumerator0
          _)
        (:NewEnumerator1
          (CallFunction|CEAligntoOriginalOrientation)))
      (bind _returnvalue (Utilities|Time|SetTimerbyEvent (EventDispatchers|CreateEvent :!event Custom|CE_ScaleFP) 0.01 true))
      (Variables|Timers|SetSFP_Timer _returnvalue)
      (CallFunction|CEOpenGate)
      (Variables|Validation|SetisHeld true))))

(fn ConstructionScript
  (CallFunction|GetMass)
  (CallFunction|GetScale))

(fn GetStartVariables
  (Variables|ForcedPerspective|SetStartingBounds (.BoxExtent (Collision|GetComponentBounds (Variables|Default|GetBox))))
  (Variables|ForcedPerspective|SetStartingDistanceFP (Math|Vector|Distance(Vector) "0, 0, 0" (Variables|/Script/Engine.SceneComponent|GetRelativeLocation (Variables|Default|GetBox))))
  (Variables|ForcedPerspective|SetStartingScale (Transformation|GetWorldScale (Variables|Default|GetBox)))
  (Variables|ForcedPerspective|SetStartingLocation (Transformation|GetWorldLocation (Variables|Default|GetBox))))

(fn CustomVertexTrace
  (bind _box (Variables|Default|GetBox))
  (bind _box_2 (Variables|Default|GetBox))
  (bind _parent_component (Variables|Default|GetParent%20Component))
  (bind _returnvalue (Transformation|GetWorldRotation _box))
  (bind _returnvalue_2 (Transformation|GetWorldLocation _parent_component))
  ;[0 0 0] Loop each vertex of "Custom trace object" Acts as an invisible proxy model to keep trace count low
  (bind _vertices (Class|KismetProceduralMeshLibrary|GetSectionfromStaticMesh (Variables|/Script/Engine.StaticMeshComponent|GetStaticMesh (Variables|Default|GetCustomTraceObject))))
  (for _array_element _vertices
    (bind (_outhit _returnvalue_3) (Collision|LineTraceByChannel (.OutputPin (CallFunction|GetFPTraceStartEnd _array_element)) (.ReturnValue (CallFunction|GetFPTraceStartEnd _array_element)) "TraceTypeQuery1" true (Utilities|Array|MakeArray self (Variables|Classes|GetInteractor)) "None"))
    (if _returnvalue_3
      ;[0 0 0] Compare impact of trace against the parent component to see if the distance is less than our current allowed closest distance
      (if (< (Math|Vector|Distance(Vector) (Transformation|GetWorldLocation (Variables|Default|GetParent%20Component)) (.ImpactPoint (Collision|BreakHitResult _outhit))) (Variables|ForcedPerspective|GetClosestDistance))
        (Variables|ForcedPerspective|SetClosestDistance (Math|Vector|Distance(Vector) (Transformation|GetWorldLocation (Variables|Default|GetParent%20Component)) (.ImpactPoint (Collision|BreakHitResult _outhit))))
        ;[0 0 0] If the scale type is align to original rotation - set world rotation to 0,0,0
        (switch Utilities|FlowControl|Switch|SwitchonE_ScalingTypes (Variables|Editable|GetScaleTypes)
          (:NewEnumerator1
            (if (not (Variables|Validation|GetAligning))
              (Transformation|SetWorldRotation (Variables|Default|GetBox) "0, 0, 0" false false)))))))
  (if (Math|Boolean|ORBoolean (> (.roll _returnvalue) 45.0) (< (.roll _returnvalue) -45.0) (> (.pitch _returnvalue) 45.0) (< (.pitch _returnvalue) -45.0))
    (Variables|ForcedPerspective|SetCustomDistance 0.75)
    (else
      (Variables|ForcedPerspective|SetCustomDistance 0.95)))
  ;[0 0 0] Call our smooth transition to position the actor at the desired held point
  (CallFunction|SmoothTransition)
  ;[0 0 0] Set new world location of the Actor
  (Transformation|SetWorldLocation _box_2 (+ _returnvalue_2 (* (Math|Vector|Lerp(Vector) (Math|Vector|GetUnitDirection(Vector) _returnvalue_2 (Transformation|GetWorldLocation (Variables|Default|GetBox))) (Math|Vector|GetForwardVector _parent_component) (Variables|ForcedPerspective|GetTransitionAlpha)) (* (Variables|ForcedPerspective|GetClosestDistance) (Variables|ForcedPerspective|GetCustomDistance)))) false false)
  (Transformation|SetWorldScale3D _box_2 (Math|Vector|ClampVectorSize (/ (* (Variables|ForcedPerspective|GetStartingScale) (/ (* (Variables|ForcedPerspective|GetClosestDistance) (Variables|ForcedPerspective|GetCustomDistance)) (Variables|ForcedPerspective|GetStartingDistanceFP))) (Transformation|GetWorldScale (Variables|Default|GetScale%20Component))) 0.1 1e+01))
  ;[0 0 0] Use the final result of our scale as a muliplier for the actors mass
  (bind _output_get (Variables|ForcedPerspective|SetFinalScale (Math|Vector|ClampVectorSize (/ (* (Variables|ForcedPerspective|GetStartingScale) (/ (* (Variables|ForcedPerspective|GetClosestDistance) (Variables|ForcedPerspective|GetCustomDistance)) (Variables|ForcedPerspective|GetStartingDistanceFP))) (Transformation|GetWorldScale (Variables|Default|GetScale%20Component))) 0.1 1e+01)))
  (Variables|Mass|SetMass (* (Variables|Mass|GetStartingMass) (.x _output_get)))
  (Variables|ForcedPerspective|SetClosestDistance 5e+06))

(fn GetMass
  (bind _box (Variables|Default|GetBox))
  (bind _returnvalue (Physics|GetMass _box))
  ;[0 0 0] Get Starting Mass - Set Custom Mass
  (Variables|Mass|SetStartingMass _returnvalue)
  (Variables|Mass|SetMass _returnvalue))

(fn SetMass
  ;[0 0 0] Set Mass Override With Custom Mass
  (Class|PrimitiveComponent|SetMassOverrideinKg (Variables|Default|GetBox) "None" (Variables|Mass|GetMass) true))

(fn GetScale
  (Variables|ForcedPerspective|SetFinalScale (Transformation|GetWorldScale (Variables|Default|GetBox))))

(fn GetPickupBaseVariables
  (params (Interactor :type Actor%20Object%20Reference) (Interactor%20Component :type Actor%20Component%20Object%20Reference))
  (Variables|Classes|SetInteractor Interactor)
  (Variables|Default|SetInteractor%20Component Interactor%20Component)
  (Class|BPIPlayerChecks|SetHeldObject(Message) (Variables|Classes|GetInteractor) (Variables|Default|GetBox))
  (Input|EnableInput (Game|GetPlayerController 0))
  (bind _scalecomponent (Class|BPIPlayerChecks|GetScaleComponent(Message) (Variables|Classes|GetInteractor)))
  (Variables|Default|SetScale%20Component _scalecomponent)
  (bind _max_range (Class|BPIComponentChecks|GetTraceLength(Message) (Variables|Default|GetInteractor%20Component)))
  (Variables|ForcedPerspective|SetMax%20Range _max_range)
  (bind _parentcomponent (Class|BPIPlayerChecks|GetPickupComponent(Message) (Variables|Classes|GetInteractor)))
  (Variables|Default|SetParent%20Component _parentcomponent)
  (return))

(fn GetFPTraceStartEnd
  (params (InputPin :type Vector))
  (bind _parent_component (Variables|Default|GetParent%20Component))
  (bind _returnvalue (Transformation|GetWorldLocation _parent_component))
  (return _returnvalue (+ _returnvalue (* (Math|Vector|GetUnitDirection(Vector) _returnvalue (Math|Transform|TransformLocation (Transformation|GetWorldTransform (Variables|Default|GetCustomTraceObject)) InputPin)) (Variables|ForcedPerspective|GetMaxRange)))))

(fn GetActorInteractor
  (return self (Variables|Default|GetCollision)))

(fn GetFPActor
  (return (Variables|Default|GetBox) self))

(fn GetObjectMass
  (return (Physics|GetMass (Variables|Default|GetBox))))

(fn GetPhysicsHandle
  (return 0))

(fn GetPickupComponent
  (return 0))

(fn GetPlayer
  (return 0))

(fn GetScaleComponent
  (return 0))

(fn GetTransitionVariables
  (return 0))

(fn IsHoldingObject
  (return false))

(fn IsObjectHeld
  (return (Variables|Validation|GetisHeld)))

(fn SetHeldObject
  (params (Component :type Primitive%20Component%20Object%20Reference))
  (return 0))