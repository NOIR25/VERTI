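; Door actor for the interaction system that swings open when OpenDoor is called, with no closing logic.
; OpenDoor clears the block through CE_ToggleBlock, which triggers CE_OpenDoor to play the DoorOpen timeline from the start.
; The timeline lerps the Door component's yaw from its current value toward a fixed open angle on each update.
; GetFPActor, GetObjectMass, GetTransitionVariables and IsObjectHeld are stubs returning empty or default values.
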(event Custom|CE_ToggleBlock
  (params (Block :type Boolean))
  ;[0 0 0] Call Open Door
  (if (not Block)
    (CallFunction|CEOpenDoor)))

(event Custom|CE_OpenDoor
  (bind _door (Variables|Default|GetDoor))
  (bind _relativerotation (Variables|/Script/Engine.SceneComponent|GetRelativeRotation _door))
  ;[0 0 0] Simple door open - Calls once
  (bind _alpha (Timeline|DoorOpen PlayFromStart)
    (:Update
      (Transformation|SetRelativeRotation _door (Math|Rotator|MakeRotator (.roll _relativerotation) (.pitch _relativerotation) (Math|Float|Lerp (.yaw _relativerotation) -9e+01 _alpha)) false false))))

(event EventBeginPlay)

(event EventOpenDoor
  ;[0 0 0] Call toggle block
  (CallFunction|CEToggleBlock false))

(fn ConstructionScript)

(fn GetFPActor
  (return 0 0))

(fn GetObjectMass
  (return 0.0))

(fn GetTransitionVariables
  (return 0))

(fn IsObjectHeld
  (return false))