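; Bookshelf puzzle actor that, when unlocked, reveals a hidden mesh and slides the shelf to a target location.
; TriggerUnlock makes the mesh visible and collidable, removes the prompt widget and trigger, plays two sounds, then runs the DoorOpen timeline.
; The timeline lerps from the shelf's current position each update rather than a cached start.
; Player overlap toggles the widget, and interaction getters are stubs except GetTransitionVariables, which returns PositionActor.
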(event OnComponentBeginOverlap(Collision)
  (params (OverlappedComponent :type Primitive%20Component%20Object%20Reference) (OtherActor :type Actor%20Object%20Reference) (OtherComp :type Primitive%20Component%20Object%20Reference) (OtherBodyIndex :type Integer) (bFromSweep :type Boolean) (SweepResult :type Hit%20Result%20Structure%20%28by%20ref%29))
  (bind _widget (Variables|Default|GetWidget))
  ;[0 0 0] Overlap to toggle UI - Replace Cast with interface implementation
  (Utilities|Casting|CastToBP_MainPlayer OtherActor)
  (Utilities|IsValid _widget
    (:Is%20Valid
      (Rendering|SetVisibility _widget true false))))

(event OnComponentEndOverlap(Collision)
  (params (OverlappedComponent :type Primitive%20Component%20Object%20Reference) (OtherActor :type Actor%20Object%20Reference) (OtherComp :type Primitive%20Component%20Object%20Reference) (OtherBodyIndex :type Integer))
  (bind _widget (Variables|Default|GetWidget))
  ;[0 0 0] Overlap to toggle UI - Replace Cast with interface implementation
  (Utilities|Casting|CastToBP_MainPlayer OtherActor)
  (Utilities|IsValid _widget
    (:Is%20Valid
      (Rendering|SetVisibility _widget false false))))

(event Custom|CE_ToggleBlock
  (params (Block :type Boolean))
  (bind _meshtoappear (Variables|Default|GetMeshToAppear))
  (bind _meshtoappear_2 (Variables|Default|GetMeshToAppear))
  ;[0 0 0] Toggle Block - Accepting puzzle solution
  (if Block
    (Rendering|SetVisibility _meshtoappear_2 false false)
    (Collision|SetCollisionEnabled _meshtoappear_2 "NoCollision")
    (else
      (Rendering|SetVisibility _meshtoappear true false)
      (Collision|SetCollisionEnabled _meshtoappear "QueryAndPhysics")
      (CallFunction|CEMoveBOokshelf))))

(event Custom|CE_MoveBookshelf
  ;[0 0 0] Move Bookshelf
  (Components|DestroyComponent (Variables|Default|GetWidget))
  (Audio|PlaySoundatLocation "/Game/Assets/SFX/general/Beeps/Correct_Cue.Correct_Cue" (Transformation|GetWorldLocation (Variables|Default|GetBookShelf)) "0, 0, 0" 1.0 1.0 0.0 0 0 0 0)
  (Audio|PlaySoundatLocation "/Game/Assets/SFX/Dialogue/Narration/AINowGetOut.AINowGetOut" (Variables|Vectors|GetLocation) "0, 0, 0" 1.0 1.0 0.0 0 0 0 0)
  (bind _alpha (Timeline|DoorOpen Play)
    (:Update
      (Transformation|SetRelativeLocation (Variables|Default|GetBookShelf) (Math|Vector|Lerp(Vector) (Variables|/Script/Engine.SceneComponent|GetRelativeLocation (Variables|Default|GetBookShelf)) (Variables|Vectors|GetMoveToLocation) _alpha) false false))))

(event EventTriggerUnlock
  ;[0 0 0] Trigger Unblock
  (CallFunction|CEToggleBlock false))

(fn ConstructionScript)

(fn GetFPActor
  (return 0 0))

(fn GetObjectMass
  (return 0.0))

(fn GetTransitionVariables
  (return (Variables|Default|GetPositionActor)))

(fn IsObjectHeld
  (return false))