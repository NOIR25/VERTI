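; BP_NewLocationTrigger is an interaction-system actor that shows a location intro on the HUD.
; Its CallNewLocation event passes through a DoOnce, then calls CallLocationIntro on the HUD held by ACLocationTriggerBehaviour, passing Location and Speed as the time.
; The remaining functions, such as GetObjectMass and IsObjectHeld, are stubs returning empty or default values.
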(event EventCallNewLocation
  ;[0 0 0] Call animation on HUD widget
  (Utilities|FlowControl|DoOnce false
    (:Completed
      (Default|CallLocationIntro (Variables|/Game/Classes/Blueprints/InteractionSystem/ComponentLibrary/Interactables/AC_LocationTriggerBehaviour.AC_LocationTriggerBehaviour_C|GetBP_HUD (Variables|Default|GetAC_LocationTriggerBehaviour)) (Variables|Default|GetLocation) (Variables|Default|GetSpeed)))))

(fn ConstructionScript)

(fn GetFPActor
  (return 0 0))

(fn GetObjectMass
  (return 0.0))

(fn GetTransitionVariables
  (return 0))

(fn IsObjectHeld
  (return false))