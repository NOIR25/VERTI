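; Template light actor for the interaction system, with a point light that can be switched on and off.
; ToggleLight uses a FlipFlop to alternate the PointLight's visibility, showing it on the first call regardless of its starting state.
; The first-person actor, object mass, transition variable and held-state queries are stubs returning empty or default values.
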(event EventToggleLight
  (bind _pointlight (Variables|Default|GetPointLight))
  (Utilities|FlowControl|FlipFlop
    (:A
      (Rendering|SetVisibility _pointlight true false))
    (:B
      (Rendering|SetVisibility _pointlight false false))))

(fn ConstructionScript)

(fn GetFPActor
  (return 0 0))

(fn GetObjectMass
  (return 0.0))

(fn GetTransitionVariables
  (return 0))

(fn IsObjectHeld
  (return false))