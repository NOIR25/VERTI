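; Template door actor for the interaction system that opens by moving its Interactable component vertically.
; The OpenDoor event plays the Door timeline, whose Alpha track sets the component's relative Z directly while preserving X and Y.
; There is no closing logic, and the functions for first-person actor, object mass, transition variables and held state are stubs returning empty or default values.
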(event EventBeginPlay)

(event Collision|EventActorBeginOverlap
  (params (OtherActor :type Actor%20Object%20Reference)))

(event EventTick
  (params (DeltaSeconds :type Float%20%28single-precision%29)))

(event EventOpenDoor
  (bind _interactable (Variables|Default|GetInteractable))
  (bind _relativelocation (Variables|/Script/Engine.SceneComponent|GetRelativeLocation _interactable))
  (bind _alpha (Timeline|Door Play)
    (:Update
      (Transformation|SetRelativeLocation _interactable (Math|Vector|MakeVector (.x _relativelocation) (.y _relativelocation) _alpha) false false))))

(fn ConstructionScript)

(fn GetFPActor
  (return 0 0))

(fn GetObjectMass
  (return 0.0))

(fn GetTransitionVariables
  (return 0))

(fn IsObjectHeld
  (return false))